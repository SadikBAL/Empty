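; BP_Spawner builds a maze in the level on BeginPlay from a Maze node graph, starting at the start node.
; SpawnNode recursively walks Up, Down, Left and Right neighbours, using the Spawned list to skip visited nodes.
; Each node spawns its own BP_Tile, offset half a room from the parent's edge, and receives its node data.
; Spawned GUIDs and their count are printed for debugging; older class-based spawning logic is left unconnected.
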(event `self.ReceiveBeginPlay`
  (bind _spawned (`self.Spawned`))
  (`|ExecutionSequence`
    (:`then_0`
      (`KismetArrayLibrary.Array_Clear` (`self.Spawned`))
      (`self.Spawn Node` (`ProceduralLevelGraphRuntime.StartNode` (`self.Maze`)) "None"))
    (:`then_1`
      (for _array_element _spawned
        (`KismetSystemLibrary.PrintString` (`KismetGuidLibrary.Conv_GuidToString` (`MazeNodeBase.NodeGuid` _array_element)) true true (struct :`R` 1.0 :`G` 0.20615 :`A` 1.0) 5.0))
      (`KismetSystemLibrary.PrintString` (`KismetStringLibrary.Conv_IntToString` (`KismetArrayLibrary.Array_Length` _spawned)) true true (struct :`R` 1.0 :`G` 0.006156 :`B` 0.004166 :`A` 1.0) 5.0))))

(fn `Spawn Bluprint`
  (params (Node :type "MazeNodeBase Object Reference") (StartLocation :type "Vector Structure"))
  (returns (EndLocation :type "Vector Structure")))

(fn `Spawn Node`
  (params (MazePart :type "MazeNodeBase Object Reference") (Direct :type "EMazeDirection Enum" :default "Up") (Location :type "Vector Structure"))
  (bind _upnode (`MazeNodeBase.UpNode` MazePart))
  (bind _downnode (`MazeNodeBase.DownNode` MazePart))
  (bind _leftnode (`MazeNodeBase.LeftNode` MazePart))
  (bind _rightnode (`MazeNodeBase.RightNode` MazePart))
  (if (< (`KismetArrayLibrary.Array_Find` (`self.Spawned`) MazePart) 0)
    (`KismetArrayLibrary.Array_Add` (`self.Spawned`) MazePart)
    (switch `EMazeDirection` Direct
      (:`Up`
        (bind _returnvalue (`MazeNodeBase.GetHalfDistanceOfRoom` MazePart "Vertical"))
        (bind _returnvalue_2 (`MazeNodeBase.SpawnMazeObject` MazePart self (+ Location (`KismetMathLibrary.MakeVector` 0.0 _returnvalue))))
        (bind _asbp_tile (cast `/Game/LevelPrototyping/BP_Tile` _returnvalue_2))
        (`/Game/LevelPrototyping/BP_Tile.SetNodeData` _asbp_tile MazePart))
      (:`Down`
        (bind _returnvalue_3 (`MazeNodeBase.GetHalfDistanceOfRoom` MazePart "Vertical"))
        (bind _returnvalue_4 (`MazeNodeBase.SpawnMazeObject` MazePart self (- Location (`KismetMathLibrary.MakeVector` 0.0 _returnvalue_3))))
        (bind _asbp_tile_2 (cast `/Game/LevelPrototyping/BP_Tile` _returnvalue_4))
        (`/Game/LevelPrototyping/BP_Tile.SetNodeData` _asbp_tile_2 MazePart))
      (:`Left`
        (bind _returnvalue_5 (`MazeNodeBase.GetHalfDistanceOfRoom` MazePart "Horizontal"))
        (bind _returnvalue_6 (`MazeNodeBase.SpawnMazeObject` MazePart self (- Location (`KismetMathLibrary.MakeVector` _returnvalue_5))))
        (bind _asbp_tile_3 (cast `/Game/LevelPrototyping/BP_Tile` _returnvalue_6))
        (`/Game/LevelPrototyping/BP_Tile.SetNodeData` _asbp_tile_3 MazePart))
      (:`Right`
        (bind _returnvalue_7 (`MazeNodeBase.GetHalfDistanceOfRoom` MazePart "Horizontal"))
        (bind _returnvalue_8 (`MazeNodeBase.SpawnMazeObject` MazePart self (+ Location (`KismetMathLibrary.MakeVector` _returnvalue_7))))
        (bind _asbp_tile_4 (cast `/Game/LevelPrototyping/BP_Tile` _returnvalue_8))
        (`/Game/LevelPrototyping/BP_Tile.SetNodeData` _asbp_tile_4 MazePart))
      (:`None`
        (bind _returnvalue_9 (`MazeNodeBase.SpawnMazeObject` MazePart self Location))
        (bind _asbp_tile_5 (cast `/Game/LevelPrototyping/BP_Tile` _returnvalue_9))
        (`/Game/LevelPrototyping/BP_Tile.SetNodeData` _asbp_tile_5 MazePart)))
    (`|ExecutionSequence`
      (:`then_0`
        (`/Engine/EditorBlueprintResources/StandardMacros.IsValid` _upnode
          (:`Is Valid`
            (bind _returnvalue_10 (`MazeNodeBase.GetEdgePosition` MazePart "Up"))
            (`self.Spawn Node` _upnode "Up" _returnvalue_10))))
      (:`then_1`
        (`/Engine/EditorBlueprintResources/StandardMacros.IsValid` _downnode
          (:`Is Valid`
            (bind _returnvalue_11 (`MazeNodeBase.GetEdgePosition` MazePart "Down"))
            (`self.Spawn Node` _downnode "Down" _returnvalue_11))))
      (:`then_2`
        (`/Engine/EditorBlueprintResources/StandardMacros.IsValid` _leftnode
          (:`Is Valid`
            (bind _returnvalue_12 (`MazeNodeBase.GetEdgePosition` MazePart "Left"))
            (`self.Spawn Node` _leftnode "Left" _returnvalue_12))))
      (:`then_3`
        (`/Engine/EditorBlueprintResources/StandardMacros.IsValid` _rightnode
          (:`Is Valid`
            (bind _returnvalue_13 (`MazeNodeBase.GetEdgePosition` MazePart "Right"))
            (`self.Spawn Node` _rightnode "Right" _returnvalue_13)))))))

(fn `UserConstructionScript`)